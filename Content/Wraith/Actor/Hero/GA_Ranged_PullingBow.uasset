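; Gameplay ability for the Wraith hero's held bow-aim stance, which ends when the input is released.
; Activation adds the ranged input context, switches camera data and faces the character along controller yaw; ending reverses this.
; It manually applies the initial attack cooldown and plays the aim montage, replaying it as a reload whenever an Ability.Ranged.Attack ability commits.
; A ShootArrow event montage chain is left unconnected.
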(event Ability|EventActivateAbility
  (bind _returnvalue (Ability|GetAbilitySystemComponentfromActorInfo))
  (CallFunction|HandleCameraandInputMapping true)
  ;[1 1 1] Mannually Apply Initial Ranged Attack Cooldown
  (GameplayEffects|ApplyGameplayEffectSpecToSelf _returnvalue (GameplayEffects|MakeOutgoingSpec :self _returnvalue :GameplayEffectClass "/Game/Wraith/Actor/Hero/GE_Ranged_AttackCooldown.GE_Ranged_AttackCooldown_C" :Level 1.0))
  (|WaitforAbilityCommit :WithTag "(TagName=\"Ability.Ranged.Attack\")" :TriggerOnce false
    (:then
      (|PlayMontageandWaitProxy "None" "/Game/Wraith/ThirdParty/Actor/Bow/AM_Bow_Shoot_StartAimIdle_Inplace.AM_Bow_Shoot_StartAimIdle_Inplace" 1.0 "None" true 1.0 0.0 false
        (:then
          (Ability|Tasks|WaitInputRelease false
            (:OnRelease
              (Ability|EndAbility))))))
    (:OnCommit
      ;[1 1 1] Play Reload Animation When Ranged Attack
      (|PlayMontageandWaitProxy "None" "/Game/Wraith/ThirdParty/Actor/Bow/AM_Bow_Shoot_StartAimIdle_Inplace.AM_Bow_Shoot_StartAimIdle_Inplace" 1.0 "None" true 1.0 0.0 false))))

(event Ability|EventOnEndAbility
  (params (bWasCancelled :type Boolean))
  (CallFunction|HandleCameraandInputMapping false))

(fn HandleCameraandInputMapping
  (params (OnBegin :type Boolean))
  (bind _returnvalue (Ability|GetActorInfo))
  (bind _returnvalue_2 (Class|WraithGameplayAbility|GetAvatarActorasWraithCharacter))
  (bind _returnvalue_3 (Class|WraithGameplayAbility|GetAvatarActorasWraithCharacter))
  (bind _returnvalue_4 (PlayerController|LocalPlayerSubsystems|GetEnhancedInputLocalPlayerSubsystem (.playercontroller _returnvalue)))
  (if OnBegin
    (Input|AddMappingContext _returnvalue_4 "/Game/Wraith/Actor/Hero/IMC_Ranged.IMC_Ranged" 1 (Utilities|Struct|MakeModifyContextOptions false false false))
    (Class|WraithBlueprintFunctionLibrary|SetTargetActorCameraData _returnvalue_3 "/Game/Wraith/Actor/Hero/CameraData_Ranaged.CameraData_Ranaged")
    (Variables|/Script/Engine.Pawn|SetbUseControllerRotationYaw _returnvalue_3 true)
    (Variables|/Script/Engine.CharacterMovementComponent|SetbOrientRotationToMovement (Variables|/Script/Engine.Character|GetCharacterMovement _returnvalue_3) false)
    (return)
    (else
      (Input|RemoveMappingContext _returnvalue_4 0 "(bIgnoreAllPressedKeysUntilRelease=True,bForceImmediately=False,bNotifyUserSettings=False)")
      (Class|WraithBlueprintFunctionLibrary|SetTargetActorCameraData _returnvalue_2 "/Game/Wraith/Actor/Hero/CameraData_Default.CameraData_Default")
      (Variables|/Script/Engine.Pawn|SetbUseControllerRotationYaw _returnvalue_2 false)
      (Variables|/Script/Engine.CharacterMovementComponent|SetbOrientRotationToMovement (Variables|/Script/Engine.Character|GetCharacterMovement _returnvalue_2) true))))