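; Hero gameplay ability that handles drawing and holding a bow for ranged aiming.
; On activation it switches to ranged camera data, locks character yaw to the controller and plays the bow start montage, chaining into the idle montage on blend out.
; Releasing the input ends the ability, which restores the default camera and turns off controller yaw.
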(event Ability|EventActivateAbility
  (bind _returnvalue (Class|WraithGameplayAbility|GetAvatarActorasWraithCharacter))
  (Class|WraithBlueprintFunctionLibrary|SetTargetActorCameraData _returnvalue "/Game/Wraith/Actor/Hero/CameraData_Ranaged.CameraData_Ranaged")
  (Variables|/Script/Engine.Pawn|SetbUseControllerRotationYaw _returnvalue true)
  (|PlayMontageandWaitProxy "None" "/Game/Wraith/ThirdParty/Actor/Bow/AM_Bow_Shoot_SP_Start_Root.AM_Bow_Shoot_SP_Start_Root" 1.0 "None" true 1.0 0.0 false
    (:then
      (Ability|Tasks|WaitInputRelease false
        (:OnRelease
          (Ability|EndAbility))))
    (:OnBlendOut
      (|PlayMontageandWaitProxy "None" "/Game/Wraith/ThirdParty/Actor/Bow/AM_Bow_Shoot_SP_Idle_Root.AM_Bow_Shoot_SP_Idle_Root" 1.0 "None" true 1.0 0.0 false))))

(event Ability|EventOnEndAbility
  (params (bWasCancelled :type Boolean))
  (bind _returnvalue (Class|WraithGameplayAbility|GetAvatarActorasWraithCharacter))
  (Class|WraithBlueprintFunctionLibrary|SetTargetActorCameraData _returnvalue "/Game/Wraith/Actor/Hero/CameraData_Default.CameraData_Default")
  (Variables|/Script/Engine.Pawn|SetbUseControllerRotationYaw _returnvalue false))