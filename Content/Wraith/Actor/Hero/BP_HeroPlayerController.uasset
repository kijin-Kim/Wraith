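; BP_HeroPlayerController is the hero's player controller, with number-key test hooks for driving a Wraith AI through gameplay events.
; On BeginPlay it turns on the AbilitySystem debug display through a console command.
; Keys 1 to 4 send Walk, Run, Sprint and melee attack input tags to the pawn of the first BP_WraithAIController found in the world.
; Each press repeats the actor search, with no validity check.
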(event EventBeginPlay
  (Development|ExecuteConsoleCommand "ShowDebug AbilitySystem" 0))

(event Input|KeyboardEvents|1
  (params (Key :type Key%20Structure :default "None"))
  (:Pressed
    (bind _outactors (Actor|GetAllActorsOfClass "/Game/Wraith/Actor/AI/BP_WraithAIController.BP_WraithAIController_C"))
    (Ability|SendGameplayEventtoActor (Pawn|GetControlledPawn (Utilities|Array|Get(acopy) _outactors)) "(TagName=\"Input.Walk\")")))

(event Input|KeyboardEvents|4
  (params (Key :type Key%20Structure :default "None"))
  (:Pressed
    (bind _outactors (Actor|GetAllActorsOfClass "/Game/Wraith/Actor/AI/BP_WraithAIController.BP_WraithAIController_C"))
    (Ability|SendGameplayEventtoActor (Pawn|GetControlledPawn (Utilities|Array|Get(acopy) _outactors)) "(TagName=\"Input.Melee.Attack\")")))

(event Input|KeyboardEvents|3
  (params (Key :type Key%20Structure :default "None"))
  (:Pressed
    (bind _outactors (Actor|GetAllActorsOfClass "/Game/Wraith/Actor/AI/BP_WraithAIController.BP_WraithAIController_C"))
    (Ability|SendGameplayEventtoActor (Pawn|GetControlledPawn (Utilities|Array|Get(acopy) _outactors)) "(TagName=\"Input.Sprint\")")))

(event Input|KeyboardEvents|2
  (params (Key :type Key%20Structure :default "None"))
  (:Pressed
    (bind _outactors (Actor|GetAllActorsOfClass "/Game/Wraith/Actor/AI/BP_WraithAIController.BP_WraithAIController_C"))
    (Ability|SendGameplayEventtoActor (Pawn|GetControlledPawn (Utilities|Array|Get(acopy) _outactors)) "(TagName=\"Input.Run\")")))

(fn ConstructionScript)