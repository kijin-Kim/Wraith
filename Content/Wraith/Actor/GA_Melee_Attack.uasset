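; Melee attack gameplay ability that plays one montage from the avatar's combo set.
; On activation it looks up the avatar's DT_CombatData row by data table ID, loads its attack montages synchronously and appends them to an array.
; A float attribute on the avatar, truncated to an integer, serves as the combo index into that array.
; The ability ends only when the montage completes, with no handling for interruption or cancellation.
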(event Ability|EventActivateAbility
  (CallFunction|LoadAttackMontagesfromDataTable)
  (|PlayMontageandWaitProxy "None" (Utilities|Array|Get(acopy) (Variables|Default|GetAttackMontages) (CallFunction|GetComboCount)) 1.0 "None" true 1.0 0.0 false
    (:OnCompleted
      (Ability|EndAbility))))

(fn LoadAttackMontagesfromDataTable
  (bind _returnvalue (Utilities|GetDataTableRow "/Game/Wraith/Actor/DT_CombatData.DT_CombatData" (Class|WraithGameplayAbility|GetAvatarActorDataTableID))
    (:then
      (for _array_element (.attackmontages _returnvalue)
        (bind _returnvalue_2 (Utilities|LoadAssetBlocking _array_element))
        (bind _asanim_montage (Utilities|Casting|CastToAnimMontage _returnvalue_2))
        (Utilities|Array|Add (Variables|Default|GetAttackMontages) _asanim_montage))
      (return))))

(fn GetComboCount
  (return (Math|Float|Truncate (.ReturnValue (Ability|Attribute|GetFloatAttribute (Ability|GetAvatarActorfromActorInfo) "(AttributeName=\"AttackComboCount\",Attribute=/Script/Wraith.WraithCombatAttributeSet:AttackComboCount,AttributeOwner=\"/Script/CoreUObject.Class'/Script/Wraith.WraithCombatAttributeSet'\")")))))